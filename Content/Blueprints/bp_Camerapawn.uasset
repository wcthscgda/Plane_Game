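; Camera pawn that orbits with click-and-drag and zooms on a spring arm.
; A click still held after a short delay sets a flag that lets the axis inputs yaw and pitch the pawn.
; Zoom inputs step the arm length by a fixed amount, without clamping.
; Click-to-focus on an actor is unfinished: its trace and timeline are disconnected and its event is empty.
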(event Custom|Movetofocusedactor
  (params (Focused%20actor :type Actor%20Object%20Reference)))

(event Input|ActionEvents|InputActionClick
  (params (Key :type Key%20Structure))
  (:Pressed
    (Utilities|FlowControl|Delay 0.3)
    (CallFunction|HandleMouseClick Key))
  (:Released
    (Variables|Default|SetbClickheld false)))

(event Input|ActionEvents|InputActionZoomin
  (params (Key :type Key%20Structure))
  (:Pressed
    (CallFunction|Zoom -2e+02)))

(event Input|ActionEvents|InputActionZoomout
  (params (Key :type Key%20Structure))
  (:Pressed
    (CallFunction|Zoom 2e+02)))

(event Input|AxisEvents|InputAxisRotateHoz
  (params (AxisValue :type Float%20%28single-precision%29))
  (if (Variables|Default|GetbClickheld)
    (Class|Actor|AddActorWorldRotation (Math|Rotator|MakeRotator 0.0 0.0 (* AxisValue (Variables|Default|GetRotationSpeed))))))

(event Input|AxisEvents|InputAxisRotateVert
  (params (AxisValue :type Float%20%28single-precision%29))
  (if (Variables|Default|GetbClickheld)
    (Transformation|AddActorLocalRotation (Math|Rotator|MakeRotator 0.0 (* AxisValue (Variables|Default|GetRotationSpeed)) 0.0) false false)))

(fn ConstructionScript
  (Variables|Default|Setdefult%20arm%20length (Variables|/Script/Engine.SpringArmComponent|GetTargetArmLength (Variables|Default|GetSpringArm))))

(fn HandleMouseClick
  (params (Key :type Key%20Structure))
  (bind _returnvalue (Game|GetPlayerController 0))
  (bind _returnvalue_2 (Game|Player|IsInputKeyDown _returnvalue Key))
  (if _returnvalue_2
    (Variables|Default|SetbClickheld _returnvalue_2)))

(fn Zoom
  (params (ZoomSpeed :type Float%20%28single-precision%29))
  (Variables|/Script/Engine.SpringArmComponent|SetTargetArmLength (Variables|Default|GetSpringArm) (+ (Variables|/Script/Engine.SpringArmComponent|GetTargetArmLength (Variables|Default|GetSpringArm)) ZoomSpeed)))